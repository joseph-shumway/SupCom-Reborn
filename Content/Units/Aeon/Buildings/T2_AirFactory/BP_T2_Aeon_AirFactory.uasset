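; Aeon T2 air factory building that produces a T2 Aeon engineer and handles upgrade events.
; Building, also triggered by the X key, shows beam and effect meshes, spawns the engineer, and uses a timeline to move it and the effect vertically, hiding effects when finished.
; Upgrading, also triggered by the 3 key, sets a flag; finishing spawns a T2 air factory at its transform and destroys itself.
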(event Custom|Begin%20Build
  (bind _returnvalue (Transformation|GetActorLocation))
  (bind _returnvalue_2 (+ _returnvalue "0, 0,50.000000"))
  (Rendering|SetVisibility (Variables|Default|GetPS_Build_Beam) true false)
  (bind _returnvalue_3 (Game|SpawnActorfromClass "/Game/Units/Aeon/Units/T2_Engineer/BP_T2_Aeon_Engineer.BP_T2_Aeon_Engineer_C" (Math|Transform|MakeTransform _returnvalue_2 "0, 0, 0" "1,1,1") "Undefined" 0 0))
  (bind (_direction _height _buildeffectheight) (Timeline|Timeline_0 PlayFromStart)
    (:Update
      (Transformation|SetActorLocation _returnvalue_3 (+ _returnvalue_2 (Math|Vector|MakeVector 0.0 0.0 _height)) false false)
      (Transformation|SetRelativeLocation (Variables|Default|GetSK_Aeon_BuildEffect) (Math|Vector|MakeVector 0.0 0.0 _buildeffectheight) false false))
    (:Finished
      (Rendering|SetVisibility (Variables|Default|GetSK_Aeon_BuildEffect) false false))))

(event Custom|Finish%20Upgrade
  (Game|SpawnActorfromClass "BP_T2_Aeon_AirFactory_C" (Transformation|GetActorTransform) "Undefined" 0 0)
  (Actor|DestroyActor))

(event Custom|Begin%20Upgrade
  (Variables|Default|SetIsUpgrading true))

(event Custom|End%20Build
  (Rendering|SetVisibility (Variables|Default|GetPS_Build_Beam) false false))

(event Input|KeyboardEvents|X
  (params (Key :type Key%20Structure :default "AnyKey"))
  (bind _returnvalue (Transformation|GetActorLocation))
  (bind _returnvalue_2 (+ _returnvalue "0, 0,50.000000"))
  (:Pressed
    (Rendering|SetVisibility (Variables|Default|GetPS_Build_Beam) true false)
    (bind _returnvalue_3 (Game|SpawnActorfromClass "/Game/Units/Aeon/Units/T2_Engineer/BP_T2_Aeon_Engineer.BP_T2_Aeon_Engineer_C" (Math|Transform|MakeTransform _returnvalue_2 "0, 0, 0" "1,1,1") "Undefined" 0 0))
    (bind (_direction _height _buildeffectheight) (Timeline|Timeline_0 PlayFromStart)
      (:Update
        (Transformation|SetActorLocation _returnvalue_3 (+ _returnvalue_2 (Math|Vector|MakeVector 0.0 0.0 _height)) false false)
        (Transformation|SetRelativeLocation (Variables|Default|GetSK_Aeon_BuildEffect) (Math|Vector|MakeVector 0.0 0.0 _buildeffectheight) false false))
      (:Finished
        (Rendering|SetVisibility (Variables|Default|GetSK_Aeon_BuildEffect) false false)))))

(event Input|KeyboardEvents|3
  (params (Key :type Key%20Structure :default "AnyKey"))
  (:Pressed
    (Variables|Default|SetIsUpgrading true)))

(fn ConstructionScript
  (|CallParentFunction))