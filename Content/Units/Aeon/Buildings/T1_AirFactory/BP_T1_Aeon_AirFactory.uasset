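; Tier 1 Aeon Air Factory building that animates its own construction, produces units and can upgrade to Tier 2.
; On BeginPlay, a timeline raises the mesh from below while driving the build effect's scale and a material parameter.
; BeginBuild or a Z key press spawns an Aeon Engineer, which a second timeline moves vertically alongside beam effects.
; Upgrade only sets a flag; FinishUpgrade replaces the actor with the T2 factory.
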(event Custom|Begin%20Build
  (bind _returnvalue (Transformation|GetActorLocation))
  (bind _returnvalue_2 (+ _returnvalue "0, 0,50.000000"))
  (Rendering|SetVisibility (Variables|Default|GetPS_BuildBeam) true false)
  (bind _returnvalue_3 (Game|SpawnActorfromClass "/Game/Units/Aeon/Units/T1_Engineer/BP_T1_Aeon_Engineer.BP_T1_Aeon_Engineer_C" (Math|Transform|MakeTransform _returnvalue_2 "0, 0, 0" "1,1,1") "Undefined" 0 0))
  (bind (_direction _height _buildeffectheight) (Timeline|Build PlayFromStart)
    (:Update
      (Transformation|SetActorLocation _returnvalue_3 (+ _returnvalue_2 (Math|Vector|MakeVector 0.0 0.0 _height)) false false)
      (Transformation|SetRelativeLocation (Variables|Default|GetSK_Aeon_BuildEffect) (Math|Vector|MakeVector 0.0 0.0 _buildeffectheight) false false))
    (:Finished
      (Rendering|SetVisibility (Variables|Default|GetSK_Aeon_BuildEffect) false false))))

(event Custom|Finish%20Upgrade
  (Game|SpawnActorfromClass "/Game/Units/Aeon/Buildings/T2_AirFactory/BP_T2_Aeon_AirFactory.BP_T2_Aeon_AirFactory_C" (Transformation|GetActorTransform) "Undefined" 0 0)
  (Actor|DestroyActor))

(event Custom|End%20Build
  (Rendering|SetVisibility (Variables|Default|GetPS_BuildBeam) false false))

(event EventUpgrade
  (Variables|Default|SetIsUpgrading true))

(event EventBeginPlay
  ;[1 1 1] Init Build
  (Rendering|SetVisibility (Variables|Default|GetInitBuild) true false)
  (bind (_direction _init_height _init_build_effect) (Timeline|Init%20Build PlayFromStart)
    (:Update
      (Transformation|SetRelativeLocation (Variables|Default|GetSkeletalMesh) (Math|Vector|MakeVector 0.0 0.0 (Math|Float|Lerp -9.5e+02 0.0 _init_height)) false false)
      (Transformation|SetRelativeTransform (Variables|Default|GetInitBuild) (Math|Transform|MakeTransform "0, 0, 0" "0, 0, 0" (* (Math|Vector|MakeVector _init_build_effect _init_build_effect 1.0) 3)) false false)
      (Rendering|Material|SetScalarParameterValueonMaterials (Variables|Default|GetSkeletalMesh) "BuildAlpha" _init_build_effect))
    (:Finished
      (Rendering|SetVisibility (Variables|Default|GetInitBuild) false false))))

(event Input|KeyboardEvents|Z
  (params (Key :type Key%20Structure :default "AnyKey"))
  (bind _returnvalue (Transformation|GetActorLocation))
  (bind _returnvalue_2 (+ _returnvalue "0, 0,50.000000"))
  (:Pressed
    (Rendering|SetVisibility (Variables|Default|GetPS_BuildBeam) true false)
    (bind _returnvalue_3 (Game|SpawnActorfromClass "/Game/Units/Aeon/Units/T1_Engineer/BP_T1_Aeon_Engineer.BP_T1_Aeon_Engineer_C" (Math|Transform|MakeTransform _returnvalue_2 "0, 0, 0" "1,1,1") "Undefined" 0 0))
    (bind (_direction _height _buildeffectheight) (Timeline|Build PlayFromStart)
      (:Update
        (Transformation|SetActorLocation _returnvalue_3 (+ _returnvalue_2 (Math|Vector|MakeVector 0.0 0.0 _height)) false false)
        (Transformation|SetRelativeLocation (Variables|Default|GetSK_Aeon_BuildEffect) (Math|Vector|MakeVector 0.0 0.0 _buildeffectheight) false false))
      (:Finished
        (Rendering|SetVisibility (Variables|Default|GetSK_Aeon_BuildEffect) false false)))))

(fn ConstructionScript
  (|CallParentFunction))