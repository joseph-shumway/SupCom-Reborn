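; Aeon tier 1 air factory building that raises itself on spawn, builds engineers and upgrades into the tier 2 air factory.
; A BeginPlay timeline animates mesh height, build effect and material, then opens gates for upgrade and unit requests.
; BeginBuildUnit spawns an engineer and lifts it with a Build timeline under a beam effect.
; Upgrade flags upgrading and blocks unit builds; FinishUpgrade replaces the actor with the T2 factory.
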(event Custom|Finish%20Upgrade
  ;[1 1 1] Finish Upgrade
  (Game|SpawnActorfromClass "/Game/Units/Aeon/Buildings/Factories/T2_AirFactory/BP_T2_Aeon_FactoryAir.BP_T2_Aeon_FactoryAir_C" (Transformation|GetActorTransform) "Undefined" 0 0)
  (Actor|DestroyActor))

(event Custom|End%20Build%20Unit
  ;[1 1 1] Build Unit
  (Rendering|SetVisibility (Variables|Default|GetPS_BuildBeam) false false))

(event EventUpgrade
  (bind _returnvalue (Transformation|GetActorLocation))
  (bind _returnvalue_2 (+ _returnvalue "0, 0,50.000000"))
  ;[1 1 1] Begin Upgrade
  (Utilities|FlowControl|Gate true
    (:Exit
      (Variables|Default|SetIsUpgrading true)
      ;[1 1 1] Build Unit
      (Utilities|FlowControl|Gate true) ; enters at Close
    )))

(event EventBeginBuildUnit
  (bind _returnvalue (Transformation|GetActorLocation))
  (bind _returnvalue_2 (+ _returnvalue "0, 0,50.000000"))
  ;[1 1 1] Build Unit
  (Utilities|FlowControl|Gate true
    (:Exit
      (Rendering|SetVisibility (Variables|Default|GetPS_BuildBeam) true false)
      (bind _returnvalue_3 (Game|SpawnActorfromClass "/Game/Units/Aeon/Units/T1_Engineer/BP_T1_Aeon_Engineer.BP_T1_Aeon_Engineer_C" (Math|Transform|MakeTransform _returnvalue_2 "0, 0, 0" "1,1,1") "Undefined" 0 0))
      (bind (_direction _height _buildeffectheight) (Timeline|Build PlayFromStart)
        (:Update
          (Transformation|SetActorLocation _returnvalue_3 (+ _returnvalue_2 (Math|Vector|MakeVector 0.0 0.0 _height)) false false)
          (Transformation|SetRelativeLocation (Variables|Default|GetBP_Aeon_BuildLiquid) (Math|Vector|MakeVector 0.0 0.0 _buildeffectheight) false false))
        (:Finished
          (CallFunction|EndBuildUnit))))))

(event EventBeginPlay
  (bind _returnvalue (Transformation|GetActorLocation))
  (bind _returnvalue_2 (+ _returnvalue "0, 0,50.000000"))
  ;[1 1 1] Self Build
  (Variables|Default|SetUnitIconsList (Utilities|Array|MakeArray "/Game/UI/GameUI/Aeon/Icons/T_UAL0105_icon.T_UAL0105_icon"))
  (Rendering|SetVisibility (Variables|Default|GetInitBuild) true false)
  (bind (_direction _init_height _init_build_effect) (Timeline|TL_Init%20Build PlayFromStart)
    (:Update
      (Transformation|SetRelativeLocation (Variables|Character|GetMesh) (Math|Vector|MakeVector 0.0 0.0 (Math|Float|Lerp -9.5e+02 0.0 _init_height)) false false)
      (Transformation|SetRelativeTransform (Variables|Default|GetInitBuild) (Math|Transform|MakeTransform "0, 0, 0" "0, 0, 0" (* (Math|Vector|MakeVector _init_build_effect _init_build_effect 1.0) 3)) false false)
      (Rendering|Material|SetScalarParameterValueonMaterials (Variables|Character|GetMesh) "BuildAlpha" _init_build_effect))
    (:Finished
      (Utilities|FlowControl|Sequence
        (:then_0
          ;[1 1 1] Begin Upgrade
          (Utilities|FlowControl|Gate true) ; enters at Open
        )
        (:then_1
          ;[1 1 1] Build Unit
          (Utilities|FlowControl|Gate true) ; enters at Open
        )))))

(fn ConstructionScript
  (|CallParentFunction))