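; Aeon tier 2 land factory building that builds T2 engineers and upgrades into the T3 land factory.
; BeginBuildUnit spawns an engineer and shows beam effects while a Timeline animates the height of both unit and effect mesh, then EndBuildUnit hides the effects.
; Upgrade sets a flag and closes the gate on new builds; FinishUpgrade spawns the T3 factory in place and destroys this one.
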(event Custom|End%20Build%20Unit
  ;[1 1 1] Build Unit
  (Rendering|SetVisibility (Variables|Default|GetSK_Aeon_BuildEffect) false false))

(event EventFinishUpgrade
  ;[1 1 1] Finish Upgrade
  (Game|SpawnActorfromClass "/Game/Units/Aeon/Buildings/Factories/T3_LandFactory/BP_T3_Aeon_FactoryLand.BP_T3_Aeon_FactoryLand_C" (Transformation|GetActorTransform) "Undefined" 0 0)
  (Actor|DestroyActor))

(event EventUpgrade
  (bind _returnvalue (Transformation|GetActorLocation))
  (bind _returnvalue_2 (+ _returnvalue "0, 0,50.000000"))
  ;[1 1 1] Begin Upgrade
  (Variables|Default|SetIsUpgrading true)
  ;[1 1 1] Build Unit
  (Utilities|FlowControl|Gate false) ; enters at Close
)

(event EventBeginBuildUnit
  (bind _returnvalue (Transformation|GetActorLocation))
  (bind _returnvalue_2 (+ _returnvalue "0, 0,50.000000"))
  ;[1 1 1] Build Unit
  (Utilities|FlowControl|Gate false
    (:Exit
      (Rendering|SetVisibility (Variables|Default|GetSK_Aeon_BuildEffect) true false)
      (bind _returnvalue_3 (Game|SpawnActorfromClass "/Game/Units/Aeon/Units/T2_Engineer/BP_T2_Aeon_Engineer.BP_T2_Aeon_Engineer_C" (Math|Transform|MakeTransform _returnvalue_2 "0, 0, 0" "1,1,1") "Undefined" 0 0))
      (bind (_direction _height _buildeffectheight) (Timeline|Timeline_0 PlayFromStart)
        (:Update
          (Transformation|SetActorLocation _returnvalue_3 (+ _returnvalue_2 (Math|Vector|MakeVector 0.0 -7e+01 _height)) false false)
          (Transformation|SetRelativeLocation (Variables|Default|GetSK_Aeon_BuildEffect) (Math|Vector|MakeVector 0.0 -7e+01 _buildeffectheight) false false))
        (:Finished
          (CallFunction|EndBuildUnit))))))

(fn ConstructionScript
  (|CallParentFunction))