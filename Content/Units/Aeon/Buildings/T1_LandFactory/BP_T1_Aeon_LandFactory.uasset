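; Aeon tier 1 land factory building that animates its construction, builds Engineers and upgrades into the T2 factory.
; On BeginPlay, a timeline drives mesh height, scale, build effect and BuildAlpha material parameter, then opens gates for upgrade and production.
; BeginBuildUnit spawns an Engineer and raises it by timeline alongside beam effects.
; Upgrade only sets IsUpgrading; FinishUpgrade spawns the T2 factory and destroys this actor.
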(event Custom|End%20Build%20Unit
  ;[1 1 1] Build Unit
  (Rendering|SetVisibility (Variables|Default|GetPS_BuildBeam) false false))

(event EventUpgrade
  ;[1 1 1] Begin Upgrade
  (Utilities|FlowControl|Gate true
    (:Exit
      (Variables|Default|SetIsUpgrading true))))

(event EventFinishUpgrade
  ;[1 1 1] Finish Upgrade
  (Game|SpawnActorfromClass "/Game/Units/Aeon/Buildings/T2_LandFactory/BP_T2_Aeon_LandFactory.BP_T2_Aeon_LandFactory_C" (Transformation|GetActorTransform) "Undefined" 0 0)
  (Actor|DestroyActor))

(event EventBeginBuildUnit
  (bind _returnvalue (Transformation|GetActorLocation))
  (bind _returnvalue_2 (+ _returnvalue "0, 0,50.000000"))
  ;[1 1 1] Build Unit
  (Utilities|FlowControl|Gate true
    (:Exit
      (Rendering|SetVisibility (Variables|Default|GetPS_BuildBeam) true false)
      (bind _returnvalue_3 (Game|SpawnActorfromClass "/Game/Units/Aeon/Units/T1_Engineer/BP_T1_Aeon_Engineer.BP_T1_Aeon_Engineer_C" (Math|Transform|MakeTransform _returnvalue_2 "0, 0, 0" "1,1,1") "Undefined" 0 0))
      (bind (_direction _height _buildeffectheight) (Timeline|Timeline_0 PlayFromStart)
        (:Update
          (Transformation|SetActorLocation _returnvalue_3 (+ _returnvalue_2 (Math|Vector|MakeVector 0.0 0.0 _height)) false false)
          (Transformation|SetRelativeLocation (Variables|Default|GetSK_Aeon_BuildEffect) (Math|Vector|MakeVector 0.0 -7e+01 _buildeffectheight) false false))
        (:Finished
          (CallFunction|EndBuildUnit))))))

(event EventBeginPlay
  (bind _returnvalue (Transformation|GetActorLocation))
  (bind _returnvalue_2 (+ _returnvalue "0, 0,50.000000"))
  ;[1 1 1] Init Build
  (Rendering|SetVisibility (Variables|Default|GetInitBuild) true false)
  (bind (_direction _init_height _init_build_effect _init_build_scale) (Timeline|Timeline_1 PlayFromStart)
    (:Update
      (Transformation|SetRelativeTransform (Variables|Default|GetSkeletalMesh) (Math|Transform|MakeTransform (Math|Vector|MakeVector 0.0 0.0 (Math|Float|Lerp -2e+02 0.0 _init_height)) "0, 0, 0" (* "1.000000,1.000000,1.000000" _init_build_scale)) false false)
      (Transformation|SetRelativeTransform (Variables|Default|GetInitBuild) (Math|Transform|MakeTransform (Math|Vector|MakeVector 0.0 0.0 (* (- _init_build_effect 1.2) 1e+02)) "0.000000, 0, 0" (* (Math|Vector|MakeVector _init_build_effect _init_build_effect 1.0) 3)) false false)
      (Rendering|Material|SetScalarParameterValueonMaterials (Variables|Default|GetSkeletalMesh) "BuildAlpha" _init_build_effect))
    (:Finished
      (Rendering|SetVisibility (Variables|Default|GetInitBuild) false false)
      (Utilities|FlowControl|Sequence
        (:then_0
          ;[1 1 1] Begin Upgrade
          (Utilities|FlowControl|Gate true) ; enters at Open
        )
        (:then_1
          ;[1 1 1] Build Unit
          (Utilities|FlowControl|Gate true) ; enters at Open
        )))))

(fn ConstructionScript
  (|CallParentFunction))