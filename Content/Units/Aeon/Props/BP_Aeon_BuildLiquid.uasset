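; Aeon build-liquid prop actor that shows a spark and cloud particle effect through PSSparkyClouds.
; The construction script passes the radius, lifetime, spawn rate and size variables to the particle system as instance parameters, multiplied by the root's world scale.
; Scalar values scale by X only and size vectors by the full scale, so the effect follows the actor's scale.
; It has no active runtime logic.
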(event EventBeginPlay)

(event Collision|EventActorBeginOverlap
  (params (OtherActor :type Actor%20Object%20Reference)))

(event EventTick
  (params (DeltaSeconds :type Float%20%28single-precision%29)))

(fn ConstructionScript
  (bind _defaultsceneroot (Variables|Default|GetDefaultSceneRoot))
  (bind _ps_sparkyclouds (Variables|Default|GetPS_SparkyClouds))
  (bind _returnvalue (Transformation|GetWorldScale _defaultsceneroot))
  (bind _returnvalue_2 (Transformation|GetWorldScale _defaultsceneroot))
  (Effects|Components|ParticleSystem|SetFloatParameter _ps_sparkyclouds "Radius" (* (Variables|ParticleSettings|GetRadius) (.x _returnvalue_2)))
  (Effects|Components|ParticleSystem|SetFloatParameter _ps_sparkyclouds "Lifetime" (* (Variables|ParticleSettings|GetLifetime) (.x _returnvalue_2)))
  (Effects|Components|ParticleSystem|SetFloatParameter _ps_sparkyclouds "SparkRate" (* (Variables|ParticleSettings|GetSparkRate) (.x _returnvalue_2)))
  (Effects|Components|ParticleSystem|SetFloatParameter _ps_sparkyclouds "CloudRate" (* (Variables|ParticleSettings|GetCloudRate) (.x _returnvalue_2)))
  (Effects|Components|ParticleSystem|SetVectorParameter _ps_sparkyclouds "SparkSize" (* _returnvalue (Variables|ParticleSettings|GetSparkSize)))
  (Effects|Components|ParticleSystem|SetVectorParameter _ps_sparkyclouds "CloudSize" (* _returnvalue (Variables|ParticleSettings|GetCloudSize))))