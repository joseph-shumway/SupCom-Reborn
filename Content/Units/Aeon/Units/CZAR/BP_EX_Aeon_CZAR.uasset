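; Blueprint for the Aeon CZAR unit that plays an opening rise-and-turn motion when it begins play.
; The construction script calls the parent's, then caches the actor's starting location.
; On BeginPlay, the CZARInit timeline sets world transforms on the mesh and capsule, lifting them from that location while interpolating yaw to a quarter turn.
; Each timeline update also prints the actor location as debug output.
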(event EventBeginPlay
  (bind _alpha (Timeline|CZAR%20Init PlayFromStart)
    (:Update
      (Transformation|SetWorldTransform (Variables|Character|GetMesh) (Math|Transform|MakeTransform (+ (Math|Vector|MakeVector 0.0 0.0 (Math|Float|Lerp 0.0 5e+03 _alpha)) (Variables|Default|GetInit%20Location)) (Math|Rotator|MakeRotator 0.0 0.0 (Math|Float|Lerp 0.0 9e+01 _alpha)) "1.0,1.0,1.000000") false false)
      (Development|PrintString (Utilities|String|ToString(Vector) (Transformation|GetActorLocation))))))

(fn ConstructionScript
  (|CallParentFunction)
  (Variables|Default|SetInit%20Location (Transformation|GetActorLocation)))