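; BP_Unit is a base unit class with team coloring and a selection indicator.
; Construction tints the mesh by team color and creates a dynamic material for the selection plane.
; UpdateSelectionPlane swaps bracket textures for highlighted, selected and pressed states; highlight and deselect requests cannot override selected or pressed, so ForceDeselect clears those.
; Upgrade, FinishSpawn and BeginPlay are empty.
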(event EventBeginPlay)

(fn ConstructionScript
  (Rendering|Material|SetVectorParameterValueonMaterials (Variables|Character|GetMesh) "Team Color" (Math|Conversions|ToVector(LinearColor) (Variables|Default|GetTeamColor)))
  (bind _returnvalue (Rendering|Material|CreateDynamicMaterialInstance (Variables|Default|GetSelectionPlane) 0 "/Game/UI/GameUI/Common/Overlay/MI_SelectionPlane.MI_SelectionPlane" :!class /Script/Engine.PrimitiveComponent))
  (Variables|Default|SetDMaterialRef _returnvalue))

(fn Upgrade)

(fn UpdateSelectionPlane
  (params (SelectionStatus :type SelectionStatus%20Enum))
  (bind _dmaterialref (Variables|Default|GetDMaterialRef))
  (bind _selectionplane (Variables|Default|GetSelectionPlane))
  (switch Utilities|FlowControl|Switch|SwitchonSelectionStatus SelectionStatus
    (:NewEnumerator0
      (if (not (or (Utilities|Enum|Equal(Enum) (Variables|Default|GetSelection%20Status) "NewEnumerator3") (Utilities|Enum|Equal(Enum) (Variables|Default|GetSelection%20Status) "NewEnumerator2")))
        (Rendering|SetVisibility _selectionplane false false)))
    (:NewEnumerator1
      (if (not (or (Utilities|Enum|Equal(Enum) (Variables|Default|GetSelection%20Status) "NewEnumerator3") (Utilities|Enum|Equal(Enum) (Variables|Default|GetSelection%20Status) "NewEnumerator2")))
        (Rendering|SetVisibility _selectionplane true false :!label _label)
        (switch Utilities|FlowControl|Switch|SwitchonSelectionStatus SelectionStatus
          (:NewEnumerator1
            (Rendering|Material|SetTextureParameterValue _dmaterialref "Selection Image" "/Game/UI/GameUI/Common/Overlay/T_highlight_bracket_player_sm.T_highlight_bracket_player_sm"))
          (:NewEnumerator2
            (Rendering|Material|SetTextureParameterValue _dmaterialref "Selection Image" "/Game/UI/GameUI/Common/Overlay/T_selection_bracket_player_sm.T_selection_bracket_player_sm"))
          (:NewEnumerator3
            (Rendering|Material|SetTextureParameterValue _dmaterialref "Selection Image" "/Game/UI/GameUI/Common/Overlay/T_selection_bracket_player_md.T_selection_bracket_player_md")))))
    (:NewEnumerator2
      (Variables|Default|SetSelection%20Status "NewEnumerator2")
      (goto _label))
    (:NewEnumerator3
      (Variables|Default|SetSelection%20Status "NewEnumerator3")
      (goto _label))))

(fn ForceDeselect
  (Rendering|SetVisibility (Variables|Default|GetSelectionPlane) false false)
  (Variables|Default|SetSelection%20Status "NewEnumerator0"))

(fn FinishSpawn)